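; Pawn that picks up, carries and drops audio-bearing items, and exchanges them with a Mirror, on a single Pickup input.
; With a valid Mirror, it adds the held item or takes one out when the mirror allows; otherwise it drops the held item or grabs CloseItem.
; Carried items attach to the pawn at the Cube's position with audio on; dropped items are muted, detached and placed at a fixed height.
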(event `InputAction|Pickup`
  (params (Key :type "Key Structure"))
  (bind _closeitem (`self.CloseItem`))
  (bind _pickedupitem (`self.PickedUpItem`))
  (bind _pickedupitem_2 (`self.PickedUpItem`))
  (bind (_returnvalue_x _returnvalue_y) (`KismetMathLibrary.BreakVector` (`SceneComponent.K2_GetComponentLocation` (`self.Cube`))))
  (bind (_returnvalue_x_2 _returnvalue_y_2 _returnvalue_z) (`KismetMathLibrary.BreakVector` (`self.K2_GetActorLocation` _closeitem)))
  (bind (_returnvalue_x_3 _returnvalue_y_3 _returnvalue_z_2) (`KismetMathLibrary.BreakVector` (`SceneComponent.K2_GetComponentLocation` (`/Game/Blueprints/ItemBP.DefaultSceneRoot` _pickedupitem))))
  (:`Pressed`
    (if (`KismetSystemLibrary.IsValid` (`self.Mirror`))
      (if (`KismetSystemLibrary.IsValid` (`self.PickedUpItem`))
        (if (`/Game/Blueprints/MirrorBP.CanAddItem` (`self.Mirror`))
          ;[1 1 1] Colocar en espejo
          (set `self.ItemToAdd` (`self.PickedUpItem`))
          (`|ExecutionSequence`
            (:`then_0`
              ;[1 1 1] Soltar objeto
              (`AudioComponent.SetVolumeMultiplier` (`/Game/Blueprints/ItemBP.Audio` _pickedupitem_2) 0.0 :!label _label)
              (`self.K2_DetachFromActor` _pickedupitem_2 "KeepRelative" "KeepRelative" "KeepRelative")
              (`self.K2_SetActorLocation` (`self.PickedUpItem`) (`KismetMathLibrary.MakeVector` _returnvalue_x _returnvalue_y 80.0) false false)
              (set `self.PickedUpItem` null))
            (:`then_1`
              (`/Game/Blueprints/MirrorBP.AddItem` (`self.Mirror`) (`self.ItemToAdd`)))))
        (elif (`/Game/Blueprints/MirrorBP.CanRemoveItem` (`self.Mirror`))
          ;[1 1 1] Tomar del espejo
          (bind _newparam (`/Game/Blueprints/MirrorBP.PickItem` (`self.Mirror`)))
          (set `self.CloseItem` _newparam)
          (if (`KismetSystemLibrary.IsValid` (`self.CloseItem`)) :!label _label_2
            ;[1 1 1] Coger objeto
            (`AudioComponent.SetVolumeMultiplier` (`/Game/Blueprints/ItemBP.Audio` (`self.CloseItem`)) 1.0)
            (set `self.PickedUpItem` (`self.CloseItem`))
            (set `self.PickedItemHeight` _returnvalue_z)
            (`self.K2_AttachToActor` _closeitem self "None" "KeepRelative" "KeepRelative" "KeepRelative" false)
            (set `self.PickedItemHeight` _returnvalue_z_2)
            (`SceneComponent.K2_SetWorldLocation` (`Actor.RootComponent` _pickedupitem) (`SceneComponent.K2_GetComponentLocation` (`self.Cube`)) false false))))
      (elif (`KismetSystemLibrary.IsValid` (`self.PickedUpItem`))
        (goto _label)
        (else
          (goto _label_2))))))

(fn `UserConstructionScript`)