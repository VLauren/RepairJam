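; CameraBP is a follow camera actor that trails the first RepPawnBP found in the level.
; BeginPlay stores its starting X and Z offset from that pawn, zeroing Y.
; Each Tick rotates the offset by the pawn's forward direction and eases the camera's position toward it.
; Its yaw eases toward the pawn's through an SLerp function on RepairJamGameModeBase, keeping pitch and roll, with debug prints left in.
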(event `self.ReceiveBeginPlay`
  (bind _outactors (`GameplayStatics.GetAllActorsOfClass` "/Game/Blueprints/RepPawnBP.RepPawnBP_C"))
  (bind _output_get (set `self.Player` (`|GetArrayItem` _outactors)))
  (bind (_returnvalue_x _returnvalue_y _returnvalue_z) (`KismetMathLibrary.BreakVector` (- (`self.K2_GetActorLocation`) (`self.K2_GetActorLocation` _output_get))))
  (set `self.Offset` (`KismetMathLibrary.MakeVector` _returnvalue_x 0.0 _returnvalue_z)))

(event `self.ReceiveTick`
  (params (DeltaSeconds :type "Float (single-precision)"))
  (bind (_returnvalue_roll _returnvalue_pitch) (`KismetMathLibrary.BreakRotator` (`self.K2_GetActorRotation`)))
  (bind _player (`self.Player`))
  (bind _returnvalue (`self.GetActorForwardVector` _player))
  (bind _returnvalue_2 (`KismetMathLibrary.Conv_VectorToRotator` _returnvalue))
  (`KismetSystemLibrary.PrintString` (`KismetStringLibrary.Conv_VectorToString` _returnvalue))
  (set `self.TargetPosition` (+ (`self.K2_GetActorLocation` _player) (`KismetMathLibrary.GreaterGreater_VectorRotator` (`self.Offset`) _returnvalue_2)))
  (set `self.TargetYaw` (.yaw _returnvalue_2))
  (`self.K2_SetActorLocation` (`KismetMathLibrary.VLerp` (`self.K2_GetActorLocation`) (`self.TargetPosition`) 0.1))
  (bind _asrepair_jam_game_mode_base (cast `RepairJamGameModeBase` (`GameplayStatics.GetGameMode`)))
  (`self.K2_SetActorRotation` (`RepairJamGameModeBase.SLerp` _asrepair_jam_game_mode_base (`self.K2_GetActorRotation`) (`KismetMathLibrary.MakeRotator` _returnvalue_roll _returnvalue_pitch (`self.TargetYaw`)) 0.1))
  (`KismetSystemLibrary.PrintString` "Hello"))

(fn `UserConstructionScript`)