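; ItemBP is an item actor that registers itself with RepPawnBP pawns as their nearby item.
; On overlap begin it sets itself as the pawn's CloseItem, but only while its Cube component is visible.
; On overlap end it clears CloseItem, provided that reference still points to this item.
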(event `self.ReceiveActorBeginOverlap`
  (params (OtherActor :type "Actor Object Reference"))
  (bind _asrep_pawn_bp (cast `/Game/Blueprints/RepPawnBP` OtherActor))
  (if (`SceneComponent.IsVisible` (`self.Cube`))
    (set `/Game/Blueprints/RepPawnBP.CloseItem` self _asrep_pawn_bp)))

(event `self.ReceiveActorEndOverlap`
  (params (OtherActor :type "Actor Object Reference"))
  (bind _asrep_pawn_bp (cast `/Game/Blueprints/RepPawnBP` OtherActor))
  (if (== (`/Game/Blueprints/RepPawnBP.CloseItem` _asrep_pawn_bp) self)
    (set `/Game/Blueprints/RepPawnBP.CloseItem` null _asrep_pawn_bp)))

(fn `UserConstructionScript`)