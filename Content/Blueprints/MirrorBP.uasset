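; MirrorBP is an actor that holds up to three items as a last-in, first-out stack.
; Overlap events set or clear the Mirror reference on a RepPawnBP, so the pawn knows which mirror it is at.
; AddItem hides the item's cube, reveals the matching piece on the mirror and stores the item.
; PickItem reverses this and returns the item, with CanAddItem and CanRemoveItem exposing the count limits.
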(event `self.ReceiveActorBeginOverlap`
  (params (OtherActor :type "Actor Object Reference"))
  (bind _asrep_pawn_bp (cast `/Game/Blueprints/RepPawnBP` OtherActor))
  (set `/Game/Blueprints/RepPawnBP.Mirror` self _asrep_pawn_bp))

(event `self.ReceiveActorEndOverlap`
  (params (OtherActor :type "Actor Object Reference"))
  (bind _asrep_pawn_bp (cast `/Game/Blueprints/RepPawnBP` OtherActor))
  (if (== (`/Game/Blueprints/RepPawnBP.Mirror` _asrep_pawn_bp) self)
    (set `/Game/Blueprints/RepPawnBP.Mirror` null _asrep_pawn_bp)))

(fn `AddItem`
  (params (Item :type "/Game/Blueprints/ItemBP Object Reference"))
  (`SceneComponent.SetVisibility` (`/Game/Blueprints/ItemBP.Cube` Item) false false)
  (`SceneComponent.SetVisibility` (select `int` (`self.AddedItems`) :`0` (`self.Piece1`) :`1` (`self.Piece2`) :`2` (`self.Piece3`) :`3` null) true false)
  (switch `int` (`self.AddedItems`)
    (:`0`
      (set `self.Item1` Item))
    (:`1`
      (set `self.Item2` Item))
    (:`2`
      (set `self.Item3` Item)))
  (`/Engine/EditorBlueprintResources/StandardMacros.IncrementInt` (`self.AddedItems`)))

(fn `CanAddItem`
  (returns (NewParam :type Boolean))
  (return (< (`self.AddedItems`) 3)))

(fn `CanRemoveItem`
  (returns (NewParam :type Boolean))
  (return (> (`self.AddedItems`) 0)))

(fn `PickItem`
  (returns (NewParam :type "/Game/Blueprints/ItemBP Object Reference"))
  (bind _addeditems (`self.AddedItems`))
  (bind _returnvalue (select `int` _addeditems :`0` (`self.Item1`) :`1` (`self.Item2`) :`2` (`self.Item3`) :`3` null))
  (`SceneComponent.SetVisibility` (select `int` _addeditems :`0` null :`1` (`self.Piece1`) :`2` (`self.Piece2`) :`3` (`self.Piece3`)) false false)
  (`/Engine/EditorBlueprintResources/StandardMacros.DecrementInt` (`self.AddedItems`)
    (:`  `
      (`SceneComponent.SetVisibility` (`/Game/Blueprints/ItemBP.Cube` _returnvalue) true false)
      (return _returnvalue))))

(fn `UserConstructionScript`)